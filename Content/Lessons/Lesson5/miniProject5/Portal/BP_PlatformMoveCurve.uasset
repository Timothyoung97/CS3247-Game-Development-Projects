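; BP_PlatformMoveCurve is a platform actor that jerks along a curve and explodes when interacted with.
; On BeginPlay it caches its origin, waits a random few seconds, then plays the SuddenJerk timeline once.
; The curve scales the origin vector as an offset, so displacement depends on world position.
; Interact spawns a neon explosion emitter, destroys the actor and returns 1.
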(event `self.ReceiveBeginPlay`
  (bind _origin (`self.Origin`))
  (set `self.Origin` (`self.K2_GetActorLocation`))
  (`KismetSystemLibrary.Delay` (`KismetMathLibrary.RandomFloatInRange` 2.0 5.0))
  (bind (_direction _curve_mycurve) (`Timeline|SuddenJerk` :!via `PlayFromStart`)
    (:`Update`
      (`self.K2_SetActorLocation` (+ _origin (* _origin _curve_mycurve))))))

(fn `Interact`
  (returns (Score :type Integer))
  (`GameplayStatics.SpawnEmitterAtLocation` "/Game/Effects/Particles/Explosion/P_NeonExplosion.P_NeonExplosion" (`self.K2_GetActorLocation`))
  (`self.K2_DestroyActor`)
  (return 1))

(fn `UserConstructionScript`)