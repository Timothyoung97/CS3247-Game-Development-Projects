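; Portal-capable wall actor whose construction script scales its mesh to the set width and height, and which spawns and tracks the BP_Portal actors placed on it.
; TryAddPortal converts the requested point to wall-local space, clamps it so the portal fits within the edges, and rejects overlaps using rectangle tests against existing portals.
; Accepted portals spawn with the wall's rotation and bind to OnDestroyed to keep the tracked list current.
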(fn `ClampPointToWall`
  (params (Point :type "Float (double-precision)") (WallSize :type "Float (double-precision)") (PortalRadius :type "Float (double-precision)"))
  (returns (ReturnValue :type "Float (double-precision)"))
  (locals (Offset :type "Float (double-precision)" :default 0.0))
  (set `local.Offset` (`KismetMathLibrary.FClamp` (- (- (/ WallSize 2.0) (`local.PortalRadius`)) (`KismetMathLibrary.Abs` (`local.Point`))) -9.999999790214768e+33 0.0))
  (set `local.Offset` (* (`local.Offset`) (select `bool` (< (`local.Point`) 0.0) :`false` -1.0 :`true` 1.0 :!type "Float (single-precision)")))
  (return (- (`local.Point`) (`local.Offset`))))

(fn `ConstrainPortalToWall`
  (params (PortalY :type "Float (double-precision)") (PortalZ :type "Float (double-precision)"))
  (returns (ConstrainedY :type "Float (double-precision)") (ConstrainedZ :type "Float (double-precision)"))
  (locals (ClampedY :type "Float (double-precision)" :default 0.0) (ClampedZ :type "Float (double-precision)" :default 0.0))
  (bind _returnvalue (`self.ClampPointToWall` (`local.PortalY`) (`self.WallWidth`) (`self.PortalSize`)))
  (set `local.ClampedY` _returnvalue)
  (bind _returnvalue_2 (`self.ClampPointToWall` (`local.PortalZ`) (`self.WallHeight`) (`.RadiusZ` (`self.PortalSize`))))
  (set `local.ClampedZ` _returnvalue_2)
  (return (`local.ClampedY`) (`local.ClampedZ`)))

(fn `HasRoomForNewPortal`
  (params (NewPortalY :type "Float (double-precision)") (NewPortalZ :type "Float (double-precision)"))
  (returns (HasRoom :type Boolean))
  (bind (_radiusy _radiusz) (`self.PortalSize`))
  (bind _returnvalue (`KismetMathLibrary.MakeVector2D` _radiusy _radiusz))
  (for _array_element (`self.PortalsOnWall`)
    (bind (_returnvalue_x _returnvalue_y _returnvalue_z) (`KismetMathLibrary.BreakVector` (`KismetMathLibrary.InverseTransformLocation` (`self.GetTransform`) (`self.K2_GetActorLocation` _array_element))))
    (bind _iscolliding (`/Game/Lessons/Lesson3/miniProject3/MyFunctionLibrary.RectToRectCollision` (`KismetMathLibrary.MakeVector2D` _returnvalue_y _returnvalue_z) _returnvalue (`KismetMathLibrary.MakeVector2D` (`local.NewPortalY`) (`local.NewPortalZ`)) _returnvalue))
    (if _iscolliding
      (return false)))
  (return true))

(fn `OnPortalDestroyed`
  (params (DestroyedActor :type "Actor Object Reference"))
  (`KismetArrayLibrary.Array_RemoveItem` (`self.PortalsOnWall`) DestroyedActor))

(fn `TryAddPortal`
  (params (PortalOrigin :type "Vector Structure") (PortalA :type Boolean))
  (returns (NewPortal :type "/Game/Lessons/Lesson3/miniProject3/Portal/BP_Portal Object Reference"))
  (locals (RelativePortalOrigin :type "Vector Structure" :default (0.0 0.0 0.0)))
  (bind (_relativeportalorigin_x _relativeportalorigin_y _relativeportalorigin_z) (`KismetMathLibrary.BreakVector` (`local.RelativePortalOrigin`)))
  (bind _relativeportalorigin_x_2 (`KismetMathLibrary.BreakVector` (`local.RelativePortalOrigin`)))
  (bind (_relativeportalorigin_x_3 _relativeportalorigin_y_2 _relativeportalorigin_z_2) (`KismetMathLibrary.BreakVector` (`local.RelativePortalOrigin`)))
  (set `local.RelativePortalOrigin` (`KismetMathLibrary.InverseTransformLocation` (`self.GetTransform`) (`local.PortalOrigin`)))
  (bind (_constrainedy _constrainedz) (`self.ConstrainPortalToWall` _relativeportalorigin_y _relativeportalorigin_z))
  (set `local.RelativePortalOrigin` (`KismetMathLibrary.MakeVector` _relativeportalorigin_x_2 _constrainedy _constrainedz))
  (if (`self.HasRoomForNewPortal` _relativeportalorigin_y_2 _relativeportalorigin_z_2)
    (bind _returnvalue (`|SpawnActorFromClass` "/Game/Lessons/Lesson3/miniProject3/Portal/BP_Portal.BP_Portal_C" (`KismetMathLibrary.MakeTransform` (`KismetMathLibrary.TransformLocation` (`self.GetTransform`) (`local.RelativePortalOrigin`)) (`self.K2_GetActorRotation`)) "AlwaysSpawn" "OverrideRootScale" null (`local.PortalA`) null))
    (`KismetArrayLibrary.Array_Add` (`self.PortalsOnWall`) _returnvalue)
    (add `self.OnDestroyed` _returnvalue (`|CreateDelegate` :!event `OnPortalDestroyed`))
    (return _returnvalue)))

(fn `UserConstructionScript`
  (`SceneComponent.SetWorldScale3D` (`self.StaticMesh`) (`KismetMathLibrary.MakeVector` 1.0 (/ (`self.WallWidth`) 100.0) (/ (`self.WallHeight`) 100.0))))