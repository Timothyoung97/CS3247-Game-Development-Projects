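; BP_Target_ColorChange is a target actor whose point value changes with its randomly chosen emissive color.
; From BeginPlay, ChangeType picks red, blue or green, sets the matching penalty or reward Value, then calls itself again after a random delay.
; Interact spawns a neon explosion at a slight offset, destroys the actor and returns the current Value to the caller.
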(event `Change Type`
  (switch `int` (`KismetMathLibrary.RandomIntegerInRange` 0 2)
    (:`0`
      (`PrimitiveComponent.SetMaterial` (`self.Target`) 0 "/Game/Materials/Solids/Emissives/MI_Emissive_Red.MI_Emissive_Red")
      (set `self.Value` -5))
    (:`1`
      (`PrimitiveComponent.SetMaterial` (`self.Target`) 0 "/Game/Materials/Solids/Emissives/MI_Emissive_Blue.MI_Emissive_Blue")
      (set `self.Value` 5))
    (:`2`
      (`PrimitiveComponent.SetMaterial` (`self.Target`) 0 "/Game/Materials/Solids/Emissives/MI_Emissive_Green.MI_Emissive_Green")
      (set `self.Value` 10)))
  (`KismetSystemLibrary.Delay` (`KismetMathLibrary.RandomFloatInRange` 2.0 6.0))
  (`self.Change Type`))

(event `self.ReceiveBeginPlay`
  (`self.Change Type`))

(fn `Interact`
  (returns (Score :type Integer))
  (`GameplayStatics.SpawnEmitterAtLocation` "/Game/Effects/Particles/Explosion/P_NeonExplosion.P_NeonExplosion" (+ (`self.K2_GetActorLocation`) (-25.0 0.0 0.0)))
  (`self.K2_DestroyActor`)
  (return (`self.Value`)))

(fn `UserConstructionScript`)